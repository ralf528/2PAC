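; Test player controller Blueprint for mouse-driven outline toggling on actors.
; It shows the mouse cursor on BeginPlay, then traces under the cursor on the Visibility channel when a mouse button is pressed.
; Hit Outline_BP actors get an outline created on left click and deleted on right click.
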(event EventBeginPlay
  (Variables|/Script/Engine.PlayerController|SetbShowMouseCursor (Game|GetPlayerController 0) true))

(event Input|MouseEvents|LeftMouseButton
  (params (Key :type Key%20Structure))
  (:Pressed
    (bind _asoutline_bp (Utilities|Casting|CastToOutline_BP (.hitactor (.HitResult (Game|Player|GetHitResultUnderCursorbyChannel (Game|GetPlayerController 0) "TraceTypeQuery1" true)))))
    ;[1 1 1] 타겟bp지정
    (Default|CreateOutline _asoutline_bp)))

(event Input|MouseEvents|RightMouseButton
  (params (Key :type Key%20Structure))
  (:Pressed
    (bind _asoutline_bp (Utilities|Casting|CastToOutline_BP (.hitactor (.HitResult (Game|Player|GetHitResultUnderCursorbyChannel (Game|GetPlayerController 0) "TraceTypeQuery1" true)))))
    (Default|DeleteOutline _asoutline_bp)))

(fn ConstructionScript)