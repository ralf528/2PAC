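; Actor Blueprint that shows a static mesh and can add or remove an outline on it at runtime.
; BeginPlay applies the configured Mesh to its StaticMesh component.
; CreateOutline adds a second mesh component once, with a dynamic PP_Outline_Inst material receiving Scale, though its SetStaticMesh call passes no mesh and OutlineColor targets parameter "None".
; DeleteOutline destroys that component and clears the HasOutline guard.
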(event Custom|Create%20Outline
  (if (not (Variables|Default|GetHas%20Outline))
    (bind _returnvalue (AddComponent|AddStaticMeshComponent false (Transformation|GetWorldTransform (Variables|Default|GetStaticMesh))))
    (bind _output_get (Variables|Default|SetMesh%20Component _returnvalue))
    (Components|StaticMesh|SetStaticMesh _output_get 0)
    (bind _returnvalue_2 (Rendering|Material|CreateDynamicMaterialInstance _returnvalue 0 "/Game/Assets/Shaders/PostProcess/PP_Outline_Inst.PP_Outline_Inst" "None" :!class /Script/Engine.PrimitiveComponent))
    (Rendering|Material|SetVectorParameterValue _returnvalue_2 "None" (Variables|Default|GetOutline_Color) :!class /Script/Engine.MaterialInstanceDynamic)
    (Rendering|Material|SetScalarParameterValue _returnvalue_2 "Scale" (Variables|Default|GetScale) :!class /Script/Engine.MaterialInstanceDynamic)
    (Variables|Default|SetHas%20Outline true)))

(event Custom|Delete%20Outline
  (bind _mesh_component (Variables|Default|GetMesh%20Component))
  (Utilities|IsValid _mesh_component
    (:Is%20Valid
      (Components|DestroyComponent _mesh_component)
      (Variables|Default|SetHas%20Outline false))))

(event Collision|EventActorBeginOverlap
  (params (OtherActor :type Actor%20Object%20Reference)))

(event EventTick
  (params (DeltaSeconds :type Float%20%28single-precision%29)))

(event EventBeginPlay
  (Components|StaticMesh|SetStaticMesh (Variables|Default|GetStaticMesh) (Variables|Default|GetMesh)))

(fn ConstructionScript)